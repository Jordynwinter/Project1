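; BP_Key is a key pickup actor that the player collects by walking into it.
; When BoxCollision begins an overlap, it casts the other actor to BP_ThirdPersonCharacter_custom and adds one to that character's KeyCount, then destroys itself.
; On-screen debug prints report its existence at BeginPlay, each pickup with the new key count, and any failed cast.
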(event OnComponentBeginOverlap(BoxCollision)
  (params (OverlappedComponent :type Primitive%20Component%20Object%20Reference) (OtherActor :type Actor%20Object%20Reference) (OtherComp :type Primitive%20Component%20Object%20Reference) (OtherBodyIndex :type Integer) (bFromSweep :type Boolean) (SweepResult :type Hit%20Result%20Structure%20%28by%20ref%29))
  (bind _asbp_third_person_character_custom (Utilities|Casting|CastToBP_ThirdPersonCharacter_custom OtherActor)
    (:then
      (Development|PrintString "A Key has been picked up!" true true "(R=0.119972,G=0.395833,B=0.109267,A=1.000000)" 5.0)
      (Variables|/Game/Blueprints/BP_ThirdPersonCharacter_custom.BP_ThirdPersonCharacter_custom_C|SetKeyCount _asbp_third_person_character_custom (+ (Variables|/Game/Blueprints/BP_ThirdPersonCharacter_custom.BP_ThirdPersonCharacter_custom_C|GetKeyCount _asbp_third_person_character_custom) 1)) ; Set key count
      (Development|PrintString (Utilities|String|Append "You have " (Utilities|String|ToString(Integer) (Variables|/Game/Blueprints/BP_ThirdPersonCharacter_custom.BP_ThirdPersonCharacter_custom_C|GetKeyCount _asbp_third_person_character_custom)) " key(s).") true true "(R=0.500000,G=0.264333,B=0.013021,A=1.000000)")
      (Actor|DestroyActor) ; Destroy this key
    )
    (:CastFailed
      (Development|PrintString "Key Player Cast Failed" true true "(R=1.000000,G=0.046773,B=0.000000,A=1.000000)" 5.0))))

(event EventBeginPlay
  (Development|PrintString "This Key Exists..." true true "(R=0.583333,G=0.343283,B=0.087298,A=1.000000)"))

(fn ConstructionScript)