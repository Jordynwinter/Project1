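; Falling platform that warns, drops and returns to its starting spot when the custom third-person character enters its trigger box.
; After a short delay the cube enables physics to fall, then physics turns off and a timeline lerps it back to its saved transform.
; A Ready flag blocks retriggering until the return finishes, and material swaps show each phase alongside a printed warning.
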(event OnComponentBeginOverlap(Box)
  (params (OverlappedComponent :type Primitive%20Component%20Object%20Reference) (OtherActor :type Actor%20Object%20Reference) (OtherComp :type Primitive%20Component%20Object%20Reference) (OtherBodyIndex :type Integer) (bFromSweep :type Boolean) (SweepResult :type Hit%20Result%20Structure%20%28by%20ref%29))
  (Utilities|Casting|CastToBP_ThirdPersonCharacter_custom OtherActor)
  (CallFunction|Activate))

(event Custom|Activate
  ;[0.32 0.6979 0.3053] Activate Platform
  (if (Variables|Default|GetReady)
    (Variables|Default|SetReady false)
    (Development|PrintString "Warning! ! !" true true "(R=0.369792,G=0.000000,B=0.005270,A=1.000000)")
    (Rendering|Material|SetMaterial (Variables|Default|GetCube) 0 "/Game/StarterContent/Materials/M_Rock_Sandstone.M_Rock_Sandstone")
    (Utilities|FlowControl|Delay 1.0)
    (CallFunction|Drop)))

(event Custom|Reset
  ;[0.32 0.6979 0.3053] Reset Platform
  (Variables|Default|SetResetTransform (Transformation|GetWorldTransform (Variables|Default|GetCube)))
  (Physics|SetSimulatePhysics (Variables|Default|GetCube) false)
  (Rendering|Material|SetMaterial (Variables|Default|GetCube) 0 "/Game/StarterContent/Materials/M_Ground_Moss.M_Ground_Moss")
  (bind _float (Timeline|GoBackToStarting PlayFromStart)
    (:Update
      (Transformation|SetWorldLocationAndRotation (Variables|Default|GetCube) (.location (Math|Transform|Lerp(Transform) (Variables|Default|GetResetTransform) (Variables|Default|GetStartingTransform) _float)) (.rotation (Math|Transform|Lerp(Transform) (Variables|Default|GetResetTransform) (Variables|Default|GetStartingTransform) _float)) false false))
    (:Finished
      (Variables|Default|SetReady true)
      (Rendering|Material|SetMaterial (Variables|Default|GetCube) 0 "/Game/StarterContent/Materials/M_Ground_Grass.M_Ground_Grass"))))

(event Custom|Drop
  ;[0.5833 0.3433 0.0873] Dropping Platform
  (Physics|SetSimulatePhysics (Variables|Default|GetCube) true)
  (Rendering|Material|SetMaterial (Variables|Default|GetCube) 0 "/Game/StarterContent/Materials/M_Ground_Gravel.M_Ground_Gravel")
  (Utilities|FlowControl|Delay 3.0)
  (CallFunction|Reset))

(event EventBeginPlay
  (Variables|Default|SetStartingTransform (Transformation|GetWorldTransform (Variables|Default|GetCube))) ; Saving starting location and rotation\nof the cube
)

(fn ConstructionScript)