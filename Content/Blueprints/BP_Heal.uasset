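; BP_Heal is a held healing pickup, a can that the custom third-person character carries and consumes.
; Overlapping its trigger asks the character to pick it up, and Pickup snaps its root to the hand_r socket of the supplied mesh.
; Drop detaches it and enables physics and collision on the can.
; PrimaryAction only prints a health message, clears the character's HeldItem and destroys the actor, without changing any health value.
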(event OnComponentBeginOverlap(PickupTrigger)
  (params (OverlappedComponent :type Primitive%20Component%20Object%20Reference) (OtherActor :type Actor%20Object%20Reference) (OtherComp :type Primitive%20Component%20Object%20Reference) (OtherBodyIndex :type Integer) (bFromSweep :type Boolean) (SweepResult :type Hit%20Result%20Structure%20%28by%20ref%29))
  (bind _asbp_third_person_character_custom (Utilities|Casting|CastToBP_ThirdPersonCharacter_custom OtherActor))
  (Default|TrytoPickUp _asbp_third_person_character_custom self))

(event EventPickup
  (params (ParentMesh :type Skeletal%20Mesh%20Component%20Object%20Reference))
  ;[0.5833 0.3433 0.0873] Target to Hand
  (Transformation|AttachComponentToComponent (Variables|Default|GetDefaultSceneRoot) ParentMesh "hand_r" "SnapToTarget" "KeepRelative" "KeepRelative" true))

(event EventDrop
  ;[1 0.3961 0.547] Drop
  (Transformation|DetachFromComponent (Variables|Default|GetDefaultSceneRoot) "KeepRelative" "KeepRelative" "KeepRelative" true)
  (Physics|SetSimulatePhysics (Variables|Default|GetCan) true)
  (Collision|SetCollisionEnabled (Variables|Default|GetCan) "QueryAndPhysics"))

(event EventPrimaryAction
  (params (ref_thirdPersonCharCustom :type BP%20Third%20Person%20Character%20Custom%20Object%20Reference))
  ;[0.12 0.3958 0.1093] Use
  (Development|PrintString "+10 Health!" true true "(R=0.132265,G=0.125081,B=0.453125,A=1.000000)")
  (Variables|/Game/Blueprints/BP_ThirdPersonCharacter_custom.BP_ThirdPersonCharacter_custom_C|SetHeldItem ref_thirdPersonCharCustom 0)
  (Actor|DestroyActor))

(fn ConstructionScript)